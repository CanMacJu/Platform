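; BP_PortalFence is a platform actor that forms a resizable fence with a portal plane between an Up and a Down piece.
; The construction script scales the plane and both pieces from Width and Height, placing Up and Down half the Height either side along local X.
; The plane is inset 200 units narrower than the end pieces.
; The event graph holds only disabled default events, so the Blueprint adds no runtime logic.
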(event EventBeginPlay)

(event Collision|EventActorBeginOverlap
  (params (OtherActor :type Actor%20Object%20Reference)))

(event EventTick
  (params (DeltaSeconds :type Float%20%28single-precision%29)))

(fn ConstructionScript
  (bind _up (Variables|Default|GetUp))
  (bind _down (Variables|Default|GetDown))
  (Transformation|SetRelativeScale3D (Variables|Default|GetPortalPlane) (Math|Vector|MakeVector (/ (Variables|Default|GetHeight) 1e+02) (/ (- (Variables|Default|GetWidth) 2e+02) 1e+02) 1.0))
  (Transformation|SetRelativeLocation _down (Math|Vector|MakeVector (* (Variables|Default|GetHeight) -0.5) 0.0 0.0) false false)
  (Transformation|SetRelativeScale3D _down (Math|Vector|MakeVector 1.0 (/ (Variables|Default|GetWidth) 1e+02) 1.0))
  (Transformation|SetRelativeLocation _up (Math|Vector|MakeVector (* (Variables|Default|GetHeight) 0.5) 1.0 1.0) false false)
  (Transformation|SetRelativeScale3D _up (Math|Vector|MakeVector 1.0 (/ (Variables|Default|GetWidth) 1e+02) 1.0)))