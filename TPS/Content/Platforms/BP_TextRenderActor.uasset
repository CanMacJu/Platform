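; BP_TextRenderActor is an actor, by its name world-space text, that turns to face the player when nearby.
; It caches the first player's pawn on BeginPlay and checks its distance every Tick.
; Within a fixed range, it builds a rotation from the normalized direction to the pawn using MakeRotFromX, so it pitches as well as yaws.
; Outside that range it keeps its last rotation.
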(event EventBeginPlay
  (Variables|Default|SetPlayer (Game|Player|GetPlayerPawn 0)))

(event EventTick
  (params (DeltaSeconds :type Float%20%28single-precision%29))
  (if (<= (Math|Vector|Distance(Vector) (Transformation|GetActorLocation (Variables|Default|GetPlayer)) (Transformation|GetActorLocation)) 1.5e+03)
    (bind _output_get (Variables|Default|SetDirection (Math|Vector|Normalize (- (Transformation|GetActorLocation (Variables|Default|GetPlayer)) (Transformation|GetActorLocation)))))
    (Transformation|SetActorRotation (Math|Rotator|MakeRotfromX _output_get))))

(fn ConstructionScript)